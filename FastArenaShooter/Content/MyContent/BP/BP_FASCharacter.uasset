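; Player character Blueprint that handles HUD creation and FMOD audio for movement, jumping and weapon fire.
; BeginPlay adds speed and ammo widgets and starts the Moving event, then Tick updates the speed display and the event's Speed parameter, which Jump also receives.
; Fire input selects a rifle, shotgun or rocket launcher sound, with the Shoot parameter distinguishing loaded from empty.
; Firing here only plays audio and prints debug text.
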(event EventBeginPlay
  (bind _returnvalue (UserInterface|CreateWidget "/Game/MyContent/BP/WBP_Speed.WBP_Speed_C"))
  (bind _output_get (Variables|Default|SetSpeedWidget _returnvalue))
  (UserInterface|Viewport|AddtoViewport _output_get 0)
  (Default|SpeedFunc _output_get (Math|Vector|VectorLength (Variables|/Script/Engine.MovementComponent|GetVelocity (Variables|Character|GetCharacterMovement))))
  (bind _returnvalue_2 (UserInterface|CreateWidget "/Game/MyContent/BP/WBP_HUDMunition.WBP_HUDMunition_C"))
  (bind _output_get_2 (Variables|Default|Set_userWidgetMunition _returnvalue_2))
  (UserInterface|Viewport|AddtoViewport _output_get_2 0)
  (bind _returnvalue_3 (Class|FMODBlueprintStatics|PlayEventAttached "/Game/FMOD/Events/Character/Move/Moving.Moving" (Variables|Default|GetFMODAudio) "None" "0, 0, 0" "KeepRelativeOffset")))

(event Collision|EventActorBeginOverlap
  (params (OtherActor :type Actor%20Object%20Reference)))

(event EventTick
  (params (DeltaSeconds :type Float%20%28single-precision%29))
  (Default|SpeedFunc (Variables|Default|GetSpeedWidget) (Math|Vector|VectorLength (Variables|/Script/Engine.MovementComponent|GetVelocity (Variables|Character|GetCharacterMovement))))
  (Class|FMODAudioComponent|SetParameter (stale EventBeginPlay _returnvalue_3) "Speed" (Utilities|PourcentageSpeed)))

(event EventOnJumped
  (bind _returnvalue (Class|FMODBlueprintStatics|PlayEventAttached "/Game/FMOD/Events/Character/Move/Jump.Jump" (Variables|Default|GetFMODAudio) "None" "0, 0, 0" "KeepRelativeOffset"))
  (Class|FMODAudioComponent|SetParameter _returnvalue "Speed" (Utilities|PourcentageSpeed)))

(event Input|ActionEvents|InputActionFire
  (params (Key :type Key%20Structure :default "None"))
  (:Pressed
    (if (Utilities|Enum|Equal(Enum) (Variables|Default|Get_WeaponType) "Riffle")
      (if (> (Variables|/Script/FastArenaShooter.MyWeaponBehaviour|Get_numberOfBallLeft (.Value (Utilities|Map|Find (Variables|Default|Getweapons) "/Game/MyContent/BP/BP_RiffleWeapon.BP_RiffleWeapon_C"))) 0)
        (bind _returnvalue (Class|FMODBlueprintStatics|PlayEventAttached "/Game/FMOD/Events/Weapons/Rifle/Rifle_Shoot.Rifle_Shoot" (Variables|Default|GetFMODAudio) "None" "0, 0, 0" "KeepRelativeOffset"))
        (Class|FMODAudioComponent|SetParameter _returnvalue "Shoot" 0.5)
        (Development|PrintString "Je tire RIFLE" true true "(R=1.000000,G=0.000000,B=0.006452,A=1.000000)")
        (else
          (bind _returnvalue_2 (Class|FMODBlueprintStatics|PlayEventAttached "/Game/FMOD/Events/Weapons/Rifle/Rifle_Shoot.Rifle_Shoot" (Variables|Default|GetFMODAudio) "None" "0, 0, 0" "KeepRelativeOffset"))
          (Class|FMODAudioComponent|SetParameter _returnvalue_2 "Shoot" 1.5)
          (Development|PrintString "Plus de balle" true true "(R=1.000000,G=0.000000,B=0.006452,A=1.000000)")))
      (elif (Utilities|Enum|Equal(Enum) (Variables|Default|Get_WeaponType) "Shotgun")
        (if (> (Variables|/Script/FastArenaShooter.MyWeaponBehaviour|Get_numberOfBallLeft (.Value (Utilities|Map|Find (Variables|Default|Getweapons) "/Game/MyContent/BP/BP_WeaponShotGun.BP_WeaponShotGun_C"))) 0)
          (bind _returnvalue_3 (Class|FMODBlueprintStatics|PlayEventAttached "/Game/FMOD/Events/Weapons/Shotgun/Shotgun_Shoot.Shotgun_Shoot" (Variables|Default|GetFMODAudio) "None" "0, 0, 0" "KeepRelativeOffset"))
          (Class|FMODAudioComponent|SetParameter _returnvalue_3 "Shoot" 0.5)
          (Development|PrintString "Je tire SHOTGUN" true true "(R=0.117366,G=1.000000,B=0.000000,A=1.000000)")
          (else
            (bind _returnvalue_4 (Class|FMODBlueprintStatics|PlayEventAttached "/Game/FMOD/Events/Weapons/Shotgun/Shotgun_Shoot.Shotgun_Shoot" (Variables|Default|GetFMODAudio) "None" "0, 0, 0" "KeepRelativeOffset"))
            (Class|FMODAudioComponent|SetParameter _returnvalue_4 "Shoot" 1.5)
            (Development|PrintString "Plus de balle" true true "(R=0.117366,G=1.000000,B=0.000000,A=1.000000)")))
        (elif (Utilities|Enum|Equal(Enum) (Variables|Default|Get_WeaponType) "RocketLauncher")
          (if (> (Variables|/Script/FastArenaShooter.MyWeaponBehaviour|Get_numberOfBallLeft (.Value (Utilities|Map|Find (Variables|Default|Getweapons) "/Game/MyContent/BP/BP_RocketLauncher.BP_RocketLauncher_C"))) 0)
            (bind _returnvalue_5 (Class|FMODBlueprintStatics|PlayEventAttached "/Game/FMOD/Events/Weapons/RocketLauncher/RocketLauncher_Shoot.RocketLauncher_Shoot" (Variables|Default|GetFMODAudio) "None" "0, 0, 0" "KeepRelativeOffset"))
            (Class|FMODAudioComponent|SetParameter _returnvalue_5 "Shoot" 0.5)
            (Development|PrintString "Je tire ROCKET" true true "(R=0.890478,G=1.000000,B=0.000000,A=1.000000)")
            (else
              (bind _returnvalue_6 (Class|FMODBlueprintStatics|PlayEventAttached "/Game/FMOD/Events/Weapons/RocketLauncher/RocketLauncher_Shoot.RocketLauncher_Shoot" (Variables|Default|GetFMODAudio) "None" "0, 0, 0" "KeepRelativeOffset"))
              (Class|FMODAudioComponent|SetParameter _returnvalue_6 "Shoot" 1.5)
              (Development|PrintString "Plus de balle" true true "(R=1.000000,G=0.938499,B=0.000000,A=1.000000)"))))))))

(fn ConstructionScript)