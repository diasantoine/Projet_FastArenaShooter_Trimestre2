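; Trash mob AI enemy Blueprint that drives its animation and FMOD audio feedback.
; Tick polls damage, attack and movement flags, using DoOnce gates to trigger animations and sounds, and keeps the movement sound at the actor's location.
; Player-damage flags and shotgun, rifle or rocket hits play impact sounds.
; On death it swaps the capsule for a sprite, then destroys itself after a short delay, stopping the movement sound and playing a death sound.
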(event EventBeginPlay
  (bind _returnvalue (Class|FMODBlueprintStatics|PlayEventatLocation "/Game/FMOD/Events/Enemies/TrashMob/Trash_Move.Trash_Move" (Math|Conversions|ToTransform(Vector) (Transformation|GetActorLocation))))
  (Class|FMODBlueprintStatics|EventInstancePlay _returnvalue))

(event EventTick
  (params (DeltaSeconds :type Float%20%28single-precision%29))
  (Class|FMODBlueprintStatics|EventInstanceSetTransform (stale EventBeginPlay _returnvalue) (Math|Conversions|ToTransform(Vector) (Transformation|GetActorLocation)))
  (Utilities|FlowControl|Sequence
    (:then_0
      (if (Variables|Default|Get_onTakingDMG)
        (Utilities|FlowControl|DoOnce false :!label _label
          (:Completed
            (Components|Animation|PlayAnimation (Variables|Character|GetMesh) "/Game/MyContent/3D/Enemies/Enemy1/TrashMob_Anim_Degat.TrashMob_Anim_Degat" false)
            (Class|FMODBlueprintStatics|PlayEventAttached "/Game/FMOD/Events/Enemies/TrashMob/Trash_Hit.Trash_Hit" (Variables|Default|GetFMODAudio) "None" "0, 0, 0" "KeepRelativeOffset")))
        (else
          (Utilities|FlowControl|Sequence
            (:then_0
              (goto _label Reset))
            (:then_1
              _))))
      (if (Variables|Default|Get_onAttack)
        (Utilities|FlowControl|Sequence
          (:then_0
            (goto _label_3 Reset))
          (:then_1
            (Utilities|FlowControl|DoOnce false :!label _label_2
              (:Completed
                (Components|Animation|PlayAnimation (Variables|Character|GetMesh) "/Game/MyContent/3D/Enemies/Enemy1/TrashMob_Anim_Attaque.TrashMob_Anim_Attaque" false)
                (Class|FMODBlueprintStatics|PlayEventAttached "/Game/FMOD/Events/Enemies/TrashMob/Trash_WooshAtk.Trash_WooshAtk" (Variables|Default|GetFMODAudio) "None" "0, 0, 0" "KeepRelativeOffset")))))
        (elif (Variables|Default|Get_isMoving)
          (Utilities|FlowControl|Sequence
            (:then_0
              (goto _label_2 Reset))
            (:then_1
              (Utilities|FlowControl|DoOnce false :!label _label_3
                (:Completed
                  (Components|Animation|PlayAnimation (Variables|Character|GetMesh) "/Game/MyContent/3D/Enemies/Enemy1/TrashMob_Anim_Deplacement.TrashMob_Anim_Deplacement" true)))))
          (else
            (goto _label_2 Reset)))))
    (:then_1
      (if (Variables|Default|Get_onPlayerTakingDMG)
        (Class|FMODBlueprintStatics|PlayEventAttached "/Game/FMOD/Events/Enemies/TrashMob/Trash_Atk.Trash_Atk" (Variables|Default|GetFMODAudio) "None" "0, 0, 0" "KeepRelativeOffset")
        (Variables|Default|Set_onPlayerTakingDMG false)))
    (:then_2
      (if (Variables|Default|Get_onDeath)
        (Rendering|SetVisibility (Variables|Default|GetCapsuleComponent) false true)
        (Rendering|SetVisibility (Variables|Default|Get8_Sprite) true true)
        (Utilities|FlowControl|Delay 0.25)
        (Actor|DestroyActor)))))

(event EventDestroyed
  (Class|FMODBlueprintStatics|EventInstanceStop (stale EventBeginPlay _returnvalue) false)
  (Class|FMODBlueprintStatics|PlayEventAttached "/Game/FMOD/Events/Enemies/TrashMob/Trash_Die.Trash_Die" (Variables|Default|GetFMODAudio) "None" "0, 0, 0" "KeepRelativeOffset"))

(event Collision|EventHit
  (params (MyComp :type Primitive%20Component%20Object%20Reference) (Other :type Actor%20Object%20Reference) (OtherComp :type Primitive%20Component%20Object%20Reference) (bSelfMoved :type Boolean) (HitLocation :type Vector :default "0, 0, 0") (HitNormal :type Vector :default "0, 0, 0") (NormalImpulse :type Vector :default "0, 0, 0") (Hit :type Hit%20Result%20Structure%20%28by%20ref%29))
  (Utilities|Casting|CastToBP_ShotGunBullets Other
    (:then
      _)
    (:CastFailed
      (Utilities|Casting|CastToBP_RiffleBullet Other
        (:then
          _)
        (:CastFailed
          (Utilities|Casting|CastToBP_Rocket Other)))))
  (Class|FMODBlueprintStatics|PlayEventAttached "/Game/FMOD/Events/Enemies/TrashMob/Trash_Hit.Trash_Hit" (Variables|Default|GetFMODAudio) "None" "0, 0, 0" "KeepRelativeOffset"))

(fn ConstructionScript)