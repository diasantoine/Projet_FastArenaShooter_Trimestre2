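; BP_MyCharacterController is a character Blueprint that shows its current movement speed on screen.
; On BeginPlay it creates a WBP_Speed widget, adds it to the viewport and passes it the length of the CharacterMovement velocity.
; Tick passes that value to the widget's SpeedFunc every frame to keep it updated.
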(event EventBeginPlay
  (bind _returnvalue (UserInterface|CreateWidget "/Game/MyContent/BP/WBP_Speed.WBP_Speed_C"))
  (bind _output_get (Variables|Default|SetSpeedWidget _returnvalue))
  (UserInterface|Viewport|AddtoViewport _output_get 0)
  (Default|SpeedFunc _output_get (Math|Vector|VectorLength (Variables|/Script/Engine.MovementComponent|GetVelocity (Variables|Character|GetCharacterMovement)))))

(event Collision|EventActorBeginOverlap
  (params (OtherActor :type Actor%20Object%20Reference)))

(event EventTick
  (params (DeltaSeconds :type Float%20%28single-precision%29))
  (Default|SpeedFunc (Variables|Default|GetSpeedWidget) (Math|Vector|VectorLength (Variables|/Script/Engine.MovementComponent|GetVelocity (Variables|Character|GetCharacterMovement)))))

(fn ConstructionScript)